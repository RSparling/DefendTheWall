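; BPC_Health is a character component that tracks health and handles death.
; Its Damage event subtracts the given amount from Health and prints a debug message.
; At zero or below, it adds its Money value to the GM_Wave game mode, then calls Die on the owner's BPC_DeathEffect component.
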(event EventDamage
  (params (Ammount :type Float%20%28double-precision%29))
  (Development|PrintString "Damage Taken")
  (bind _output_get (Variables|Default|Sethealth (- (Variables|Default|Gethealth) Ammount)))
  (if (<= _output_get 0.0)
    (bind _asgm_wave (Utilities|Casting|CastToGM_Wave (Game|GetGameMode)))
    (Default|AddMoney _asgm_wave (Variables|Default|GetMoney))
    (Default|Die (Actor|GetComponentbyClass (Components|GetOwner) "/Game/Dynamic/Blueprints/Components/Character/Death/BPC_DeathEffect.BPC_DeathEffect_C"))))