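; GM_Wave is a game mode Blueprint that tracks Money and Health and keeps the on-screen game widget in sync with them.
; On BeginPlay it creates WB_Game for the first player controller and adds it to the viewport.
; AddMoney, SpendMoney and TakeDamage events adjust the values and push each result to the widget, with no bounds or game-over checks here.
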(event Custom|Add%20Money
  (params (Money :type Integer))
  (bind _output_get (Variables|Default|SetMoney (+ (Variables|Default|GetMoney) Money)))
  (Default|UpdateMoney (Variables|Default|GetWidget) _output_get))

(event Custom|TakeDamage
  (params (Ammount :type Integer))
  (bind _output_get (Variables|Default|SetHealth (- (Variables|Default|GetHealth) Ammount)))
  (Default|UpdateHealth (Variables|Default|GetWidget) _output_get))

(event Custom|Spend%20Money
  (params (Ammount :type Integer))
  (bind _output_get (Variables|Default|SetMoney (- (Variables|Default|GetMoney) Ammount)))
  (Default|UpdateMoney (Variables|Default|GetWidget) _output_get))

(event EventBeginPlay
  (bind _returnvalue (UserInterface|CreateWidget "/Game/Dynamic/Blueprints/UI/WB_Game.WB_Game_C" (Game|GetPlayerController 0)))
  (bind _output_get (Variables|Default|SetWidget _returnvalue))
  (UserInterface|Viewport|AddtoViewport _output_get 0))

(fn ConstructionScript)