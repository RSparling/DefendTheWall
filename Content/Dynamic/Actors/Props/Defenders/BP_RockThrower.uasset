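; BP_RockThrower is a defender prop that automatically throws rocks at the nearest enemy in range.
; BeginPlay sets the tick interval to the throw component's fire delay and reads damage and range bonuses from GM_Wave.
; Each tick sphere-overlaps for BP_Enemy pawns and picks the closest one's location.
; If BPCThrowRock can fire, a throw montage plays, and its notify fires from the Arrow toward that location.
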(event EventTick
  (params (DeltaSeconds :type Float%20%28single-precision%29))
  (bind _bpc_throwrock (Variables|Default|GetBPC_ThrowRock))
  (bind (_outactors _returnvalue) (Collision|SphereOverlapActors (Transformation|GetWorldLocation (Variables|Default|GetDefaultSceneRoot)) (* (Variables|Default|GetBase%20Range) (Variables|Default|GetRange%20Multiplier)) (Utilities|Array|MakeArray "ObjectTypeQuery3") "/Game/Dynamic/Actors/Enemies/BP_Enemy.BP_Enemy_C"))
  (if _returnvalue
    (bind _closest_position (CallFunction|GetClosestEnemy _outactors))
    (bind _newparam (Default|CanFireNow _bpc_throwrock))
    (if _newparam
      (Animation|Montage|PlayMontage (Variables|Default|GetSkeletalMesh) "/Game/Static/Characters/Mixamo/Shared_Animations/Montage_Throw.Montage_Throw"
        (:OnNotifyBegin
          (Default|Fire _bpc_throwrock (Transformation|GetWorldLocation (Variables|Default|GetArrow)) _closest_position (Variables|Default|GetDamage%20Multiplier) 1.0))))))

(event EventBeginPlay
  (Actor|Tick|SetActorTickInterval (Variables|/Game/Dynamic/Blueprints/Components/Weapons/BPC_ThrowRock.BPC_ThrowRock_C|GetFireDelay (Variables|Default|GetBPC_ThrowRock)))
  (bind _asgm_wave (Utilities|Casting|CastToGM_Wave (Game|GetGameMode)))
  (Variables|Default|SetDamage%20Multiplier (Variables|/Game/Dynamic/Blueprints/GameModes/GM_Wave.GM_Wave_C|GetDefender%20Damage%20Bonus _asgm_wave))
  (Variables|Default|SetRange%20Multiplier (Variables|/Game/Dynamic/Blueprints/GameModes/GM_Wave.GM_Wave_C|GetDefender%20Range%20Bonus _asgm_wave)))

(fn ConstructionScript)

(fn GetClosestEnemy
  (params (Enemies :type Array%20of%20Object%20Object%20References))
  (bind _output_get (LocalVariables|SetClosest (Math|Vector|MakeVector 1e+09 1e+09 1e+09)))
  (LocalVariables|SetClosest%20Distance (Math|Vector|Distance(Vector) _output_get (Transformation|GetActorLocation)))
  (for _array_element Enemies
    (bind _asbp_enemy (Utilities|Casting|CastToBP_Enemy _array_element))
    (if (< (Math|Vector|Distance(Vector) (Transformation|GetActorLocation _asbp_enemy) (Transformation|GetActorLocation)) (LocalVariables|GetClosest%20Distance))
      (LocalVariables|SetClosest%20Distance (Math|Vector|Distance(Vector) (Transformation|GetActorLocation _asbp_enemy) (Transformation|GetActorLocation)))
      (LocalVariables|SetClosest (Transformation|GetActorLocation _asbp_enemy))))
  (return (LocalVariables|GetClosest)))