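; BP_TestEnemy is a test enemy that advances along negative X and attacks BP_Wall actors in its path.
; Each Tick, a sphere overlap sets IsInRange, choosing between moving and damaging the closest nearby wall's health component.
; Movement speed scales with a clamped log/power formula of game time.
; The attack Delay follows the damage call with nothing after it, so damage lands every in-range Tick.
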(event EventTick
  (params (DeltaSeconds :type Float%20%28single-precision%29))
  (Variables|Default|SetDelta%20Seconds DeltaSeconds)
  (Utilities|CeckforWall)
  (if (not (Variables|Default|GetisInRange))
    (Utilities|MoveDown)
    (else
      (Utilities|AttackClosestWall)
      (Utilities|FlowControl|Delay (Variables|Default|GetAttackDelay)))))

(fn ConstructionScript)

(fn GetClosestWall
  (params (Walls :type Array%20of%20Object%20Object%20References))
  (bind _output_get (LocalVariables|SetClosest%20Pos "1000000000.000000,1000000000.000000,1000000000.000000"))
  (LocalVariables|SetClosest%20Distance (Math|Vector|Distance(Vector) _output_get (Transformation|GetActorLocation)))
  (for _array_element Walls
    (bind _asbp_wall (Utilities|Casting|CastToBP_Wall _array_element))
    (if (< (Math|Vector|Distance(Vector) (Transformation|GetActorLocation _asbp_wall) (Transformation|GetActorLocation)) (LocalVariables|GetClosest%20Distance))
      (LocalVariables|SetClosest%20Distance (Math|Vector|Distance(Vector) (Transformation|GetActorLocation _asbp_wall) (Transformation|GetActorLocation)))
      (LocalVariables|SetClosest _asbp_wall)))
  (return (LocalVariables|GetClosest)))