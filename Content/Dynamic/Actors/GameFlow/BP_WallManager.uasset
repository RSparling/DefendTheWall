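; BP_WallManager is an actor that spawns defender units on wall pieces for the wave game mode.
; Shortly after BeginPlay it registers itself with GM_Wave.
; SpawnUnit picks a random entry in its Wall array and passes the requested actor to that entry's SpawnDefender, retrying up to MaxAttempts until an index is valid.
; It checks only index validity, not whether the chosen wall can take a defender.
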(event Custom|Spawn%20Unit
  (params (ActorToSpawn :type BP%20Defender%20Class%20Reference%20%28by%20ref%29))
  (bind _wall (Variables|Default|GetWall))
  (bind _returnvalue (Utilities|Array|Length _wall))
  (bind _returnvalue_2 (Math|Random|RandomInteger _returnvalue))
  (Utilities|FlowControl|ForLoopwithBreak 0 (Variables|Default|GetMax%20Attempts) :!label _label
    (:LoopBody
      (if (Utilities|Array|IsValidIndex _wall _returnvalue_2)
        (Default|SpawnDefender (Utilities|Array|Get(acopy) _wall _returnvalue_2) ActorToSpawn)
        (goto _label Break)))))

(event EventBeginPlay
  (Utilities|FlowControl|Delay 0.01)
  (bind _asgm_wave (Utilities|Casting|CastToGM_Wave (Game|GetGameMode)))
  (Default|RegisterWallManager _asgm_wave self))

(fn ConstructionScript)