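; BP_PlayerCamera is the player's camera pawn, which throws rocks at the point under the mouse cursor.
; BeginPlay shows the cursor, adds the input mapping, equips a BPC_ThrowRock component as the current weapon and registers with GM_Wave.
; Tick deprojects the mouse and line-traces on Visibility to store the target location.
; IA_Select fires the weapon from the camera toward that target with damage and fire-speed multipliers, playing a throw sound.
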(event Input|EnhancedActionEvents|EnhancedInputActionIA_Select
  (params (ActionValue :type Boolean) (ElapsedSeconds :type Float%20%28double-precision%29) (TriggeredSeconds :type Float%20%28double-precision%29) (InputAction :type Input%20Action%20Object%20Reference :default "/Game/Static/Input/IA_Select.IA_Select"))
  (bind _currentweapon (Variables|Default|GetCurrentWeapon))
  (bind _newparam (Default|CanFireNow _currentweapon))
  (if _newparam
    (Default|Fire _currentweapon (Transformation|GetWorldLocation (Variables|Default|GetCamera)) (Variables|Default|GetTargetDestination) (Variables|Default|GetDamage%20Multiplier) (Variables|Default|GetFireSpeedMultiplier))
    (Audio|PlaySoundatLocation "/Game/Static/Sounds/throw.throw" "0, 0, 0" "0, 0, 0" 1.0 0.8 0.0 0 0 0 0)))

(event EventBeginPlay
  (bind _asplayer_controller (Utilities|Casting|CastToPlayerController (Pawn|GetController self))
    (:then
      (bind _output_get (Variables|Default|SetAs%20Player%20Controller _asplayer_controller))
      (Variables|/Script/Engine.PlayerController|SetbShowMouseCursor _output_get true)
      (Input|AddMappingContext (PlayerController|LocalPlayerSubsystems|GetEnhancedInputLocalPlayerSubsystem _output_get) "/Game/Static/Input/IMC_Player.IMC_Player" 0 "(bIgnoreAllPressedKeysUntilRelease=True,bForceImmediately=False,bNotifyUserSettings=False)")
      (bind _returnvalue (AddComponent|AddBPCThrowRock))
      (Variables|Default|SetCurrentWeapon _returnvalue)
      (Input|SetInputModeGameandUI _output_get 0 "DoNotLock" true false)
      (bind _asgm_wave (Utilities|Casting|CastToGM_Wave (Game|GetGameMode)))
      (Default|RegisterPlayer _asgm_wave self))
    (:CastFailed
      (Development|PrintText "Get Player Controller Failed"))))

(event EventTick
  (params (DeltaSeconds :type Float%20%28single-precision%29))
  ;[1 1 1] Figures out camera to mouse cursor relative to the world
  (bind _asplayer_controller (Utilities|Casting|CastToPlayerController (Pawn|GetController (Game|Player|GetPlayerPawn 0))))
  (if (.ReturnValue (Game|Player|GetMousePosition _asplayer_controller))
    (if (.ReturnValue (Class|GameplayStatics|DeprojectScreentoWorld _asplayer_controller (Math|Vector2D|MakeVector2D (.LocationX (Game|Player|GetMousePosition _asplayer_controller)) (.LocationY (Game|Player|GetMousePosition _asplayer_controller)))))
      (bind (_outhit _returnvalue) (Collision|LineTraceByChannel (.WorldPosition (Class|GameplayStatics|DeprojectScreentoWorld _asplayer_controller (Math|Vector2D|MakeVector2D (.LocationX (Game|Player|GetMousePosition _asplayer_controller)) (.LocationY (Game|Player|GetMousePosition _asplayer_controller))))) (+ (* (.WorldDirection (Class|GameplayStatics|DeprojectScreentoWorld _asplayer_controller (Math|Vector2D|MakeVector2D (.LocationX (Game|Player|GetMousePosition _asplayer_controller)) (.LocationY (Game|Player|GetMousePosition _asplayer_controller))))) (Variables|Default|GetDistance)) (Transformation|GetWorldLocation (Variables|Default|GetCamera))) "TraceTypeQuery1" true 0 "ForOneFrame"))
      (Variables|Default|SethasValidTarget _returnvalue)
      (if _returnvalue
        (Variables|Default|SetTargetDestination (.location _outhit))))))

(fn ConstructionScript)