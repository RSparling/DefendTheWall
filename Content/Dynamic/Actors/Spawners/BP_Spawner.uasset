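; Enemy spawner actor that repeatedly spawns its target class at its own location until a running spawn count passes its limit.
; After a random startup delay, it requires an injected EnemyManager, which it hands to each spawned actor.
; Each spawn gets bonus health that grows very slowly with the spawner's age.
; The loop scales its delay down after every spawn, so spawns speed up, and the count never decreases here.
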(event EventBeginPlay
  (bind _returnvalue (Actor|GetGameTimeSinceCreation))
  (Utilities|FlowControl|Delay (* (Math|Random|RandomFloat) 5.0))
  (if (Utilities|IsValid (Variables|Default|GetEnemy%20Manager))
    (Utilities|FlowControl|Delay (Variables|Default|GetSpawnDelay) :!label _label)
    (if (<= (- (Variables|Default|GetCurrentSpawns) 1) (Variables|Default|GetMaxSpawns))
      (Utilities|FlowControl|Sequence
        (:then_0
          (bind _returnvalue_2 (Game|SpawnActorfromClass (Variables|Default|GetTargetSpawn) (Math|Conversions|ToTransform(Vector) (Transformation|GetWorldLocation (Variables|Default|GetDefaultSceneRoot))) "AdjustIfPossibleButDontSpawnIfColliding" "MultiplyWithRoot" 0 0))
          (Variables|/Game/Dynamic/Actors/Enemies/BP_Enemy.BP_Enemy_C|SetManager _returnvalue_2 (Variables|Default|GetEnemy%20Manager))
          (Variables|/Game/Dynamic/Blueprints/Components/Character/BPC_Health.BPC_Health_C|Sethealth (Variables|/Game/Dynamic/Actors/Enemies/BP_Enemy.BP_Enemy_C|GetBPC_Health _returnvalue_2) (+ (Variables|/Game/Dynamic/Blueprints/Components/Character/BPC_Health.BPC_Health_C|Gethealth (Variables|/Game/Dynamic/Actors/Enemies/BP_Enemy.BP_Enemy_C|GetBPC_Health _returnvalue_2)) (/ _returnvalue (Math|Float|Power _returnvalue 0.9)))))
        (:then_1
          (Variables|Default|SetCurrentSpawns (+ (Variables|Default|GetCurrentSpawns) 1)))
        (:then_2
          (Variables|Default|SetSpawnDelay (* (Variables|Default|GetSpawnDelay) (+ 0.95 (/ (Math|Random|RandomInteger 5) 100)))))
        (:then_3
          (goto _label))))))

(fn ConstructionScript)

(fn InjectManager
  (params (Enemy%20Manager :type BP%20Enemy%20Manager%20Object%20Reference))
  (Variables|Default|SetEnemy%20Manager Enemy%20Manager))