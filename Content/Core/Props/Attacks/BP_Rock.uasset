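; BP_Rock is an attack prop that damages enemies it touches.
; An overlap on its sphere collider prints the other actor's names, then applies a fixed amount of damage through the health component of a BP_Enemy and destroys the rock.
; A delay started at BeginPlay destroys the rock after its lifetime runs out.
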(event OnComponentBeginOverlap(SphereCollider)
  (params (OverlappedComponent :type Primitive%20Component%20Object%20Reference) (OtherActor :type Actor%20Object%20Reference) (OtherComp :type Primitive%20Component%20Object%20Reference) (OtherBodyIndex :type Integer) (bFromSweep :type Boolean) (SweepResult :type Hit%20Result%20Structure%20%28by%20ref%29))
  (Development|PrintString (Utilities|GetDisplayName OtherActor))
  (Development|PrintString (Utilities|GetObjectName OtherActor))
  (bind _asbp_enemy (Utilities|Casting|CastToBP_Enemy OtherActor))
  (Utilities|IsValid _asbp_enemy
    (:Is%20Valid
      (Default|Damage (Variables|/Game/Core/Enemies/BP_Enemy.BP_Enemy_C|GetBPC_Health _asbp_enemy) 1e+01)
      (Actor|DestroyActor))))

(event EventBeginPlay
  (Utilities|FlowControl|Delay 1e+01)
  (Actor|DestroyActor))

(fn ConstructionScript)