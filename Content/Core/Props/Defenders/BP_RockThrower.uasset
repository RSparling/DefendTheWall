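; BP_RockThrower is a defender prop that automatically throws rocks at the nearest enemy within range.
; BeginPlay sets the actor's tick interval to the BPCThrowRock fire delay, so Tick itself paces the attacks.
; Each tick runs a sphere overlap for BP_Enemy pawns, and GetClosestEnemy returns the nearest one's location.
; BPCThrowRock then fires from the Arrow component toward that position.
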(event EventTick
  (params (DeltaSeconds :type Float%20%28single-precision%29))
  (bind (_outactors _returnvalue) (Collision|SphereOverlapActors (Transformation|GetWorldLocation (Variables|Default|GetDefaultSceneRoot)) (Variables|Default|GetRange) (Utilities|Array|MakeArray "ObjectTypeQuery3") "/Game/Core/Enemies/BP_Enemy.BP_Enemy_C"))
  (if _returnvalue
    (bind _closest_position (CallFunction|GetClosestEnemy _outactors))
    (Default|Fire (Variables|Default|GetBPC_ThrowRock) (Transformation|GetWorldLocation (Variables|Default|GetArrow)) _closest_position)))

(event EventBeginPlay
  (Actor|Tick|SetActorTickInterval (Variables|/Game/Core/Components/Weapons/BPC_ThrowRock.BPC_ThrowRock_C|GetFireDelay (Variables|Default|GetBPC_ThrowRock))))

(fn ConstructionScript)

(fn GetClosestEnemy
  (params (Enemies :type Array%20of%20Object%20Object%20References))
  (bind _output_get (LocalVariables|SetClosest (Math|Vector|MakeVector 1e+09 1e+09 1e+09)))
  (LocalVariables|SetClosest%20Distance (Math|Vector|Distance(Vector) _output_get (Transformation|GetActorLocation)))
  (for _array_element Enemies
    (bind _asbp_enemy (Utilities|Casting|CastToBP_Enemy _array_element))
    (if (< (Math|Vector|Distance(Vector) (Transformation|GetActorLocation _asbp_enemy) (Transformation|GetActorLocation)) (LocalVariables|GetClosest%20Distance))
      (LocalVariables|SetClosest%20Distance (Math|Vector|Distance(Vector) (Transformation|GetActorLocation _asbp_enemy) (Transformation|GetActorLocation)))
      (LocalVariables|SetClosest (Transformation|GetActorLocation _asbp_enemy))))
  (return (LocalVariables|GetClosest)))