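; BP_PlayerCamera is the player's camera pawn, which aims weapons with the mouse cursor.
; On BeginPlay it adds the player Enhanced Input mapping context and creates a throw-rock component as the current weapon.
; Each tick it deprojects the cursor and traces on Visibility, storing whether a target was hit and its location.
; The select input fires the current weapon from the camera toward the last stored location, without checking target validity.
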(event Input|EnhancedActionEvents|EnhancedInputActionIA_Select
  (params (ActionValue :type Boolean) (ElapsedSeconds :type Float%20%28double-precision%29) (TriggeredSeconds :type Float%20%28double-precision%29) (InputAction :type Input%20Action%20Object%20Reference :default "/Game/Core/Input/IA_Select.IA_Select"))
  (Default|Fire (Variables|Default|GetCurrentWeapon) (Transformation|GetWorldLocation (Variables|Default|GetCamera)) (Variables|Default|GetTargetDestination)))

(event EventBeginPlay
  (bind _asplayer_controller (Utilities|Casting|CastToPlayerController (Pawn|GetController self))
    (:then
      (bind _output_get (Variables|Default|SetAs%20Player%20Controller _asplayer_controller))
      (Input|AddMappingContext (PlayerController|LocalPlayerSubsystems|GetEnhancedInputLocalPlayerSubsystem _output_get) "/Game/Core/Input/IMC_Player.IMC_Player" 0 "(bIgnoreAllPressedKeysUntilRelease=True,bForceImmediately=False,bNotifyUserSettings=False)")
      (bind _returnvalue (AddComponent|AddBPCThrowRock))
      (Variables|Default|SetCurrentWeapon _returnvalue))
    (:CastFailed
      (Development|PrintText "Get Player Controller Failed"))))

(event EventTick
  (params (DeltaSeconds :type Float%20%28single-precision%29))
  (bind _asplayer_controller (Utilities|Casting|CastToPlayerController (Pawn|GetController (Game|Player|GetPlayerPawn 0))))
  (if (.ReturnValue (Game|Player|GetMousePosition _asplayer_controller))
    (if (.ReturnValue (Class|GameplayStatics|DeprojectScreentoWorld _asplayer_controller (Math|Vector2D|MakeVector2D (.LocationX (Game|Player|GetMousePosition _asplayer_controller)) (.LocationY (Game|Player|GetMousePosition _asplayer_controller)))))
      (bind (_outhit _returnvalue) (Collision|LineTraceByChannel (.WorldPosition (Class|GameplayStatics|DeprojectScreentoWorld _asplayer_controller (Math|Vector2D|MakeVector2D (.LocationX (Game|Player|GetMousePosition _asplayer_controller)) (.LocationY (Game|Player|GetMousePosition _asplayer_controller))))) (+ (* (.WorldDirection (Class|GameplayStatics|DeprojectScreentoWorld _asplayer_controller (Math|Vector2D|MakeVector2D (.LocationX (Game|Player|GetMousePosition _asplayer_controller)) (.LocationY (Game|Player|GetMousePosition _asplayer_controller))))) (Variables|Default|GetDistance)) (Transformation|GetWorldLocation (Variables|Default|GetCamera))) "TraceTypeQuery1" true 0 "ForOneFrame"))
      (Variables|Default|SethasValidTarget _returnvalue)
      (if _returnvalue
        (Variables|Default|SetTargetDestination (.location _outhit)))
      (else
        (Development|PrintString "Deprojection Failed")))
    (else
      (Development|PrintString "No Associate Mouse Device"))))

(fn ConstructionScript)