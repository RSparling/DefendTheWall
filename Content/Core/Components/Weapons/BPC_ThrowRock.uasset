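; BPC_ThrowRock is a weapon component that throws rock projectiles from a given origin toward a target position.
; Fire, when allowed, spawns a BP_Rock, rotates it to face the target and launches it along its local forward axis at a fixed speed.
; Each throw clears CanFire and starts a cooldown that restores it after FireDelay, limiting the fire rate.
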(event EventFire
  (params (Origin :type Vector :default "0, 0, 0") (Target%20Position :type Vector :default "0, 0, 0"))
  (if (Variables|Default|GetCanFire)
    (bind _returnvalue (Game|SpawnActorfromClass "/Game/Core/Props/Attacks/BP_Rock.BP_Rock_C" (Math|Conversions|ToTransform(Vector) Origin) "Undefined" "MultiplyWithRoot" 0 0))
    (Transformation|SetActorRotation _returnvalue (Math|Rotator|FindLookatRotation Origin Target%20Position))
    (Game|Components|ProjectileMovement|SetVelocityinLocalSpace (Variables|/Game/Core/Props/Attacks/BP_Rock.BP_Rock_C|GetProjectileMovement _returnvalue) "1000.000000,0.000000,0.000000")
    (Variables|Default|SetCanFire false)
    (Utilities|BeginCooldown)))