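; BP_Spawner is a spawner actor that creates instances of TargetSpawn at its root location on a timed loop.
; BeginPlay starts the loop only if an EnemyManager is already set, which InjectManager supplies, and passes that manager to each spawned actor.
; Each pass waits SpawnDelay, spawns and increments CurrentSpawns, repeating while CurrentSpawns minus one is within MaxSpawns, so the count can exceed that limit.
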(event EventBeginPlay
  (if (!= (Variables|Default|GetEnemy%20Manager) 0)
    (Utilities|FlowControl|Delay (Variables|Default|GetSpawnDelay) :!label _label)
    (if (<= (- (Variables|Default|GetCurrentSpawns) 1) (Variables|Default|GetMaxSpawns))
      (Utilities|FlowControl|Sequence
        (:then_0
          (bind _returnvalue (Game|SpawnActorfromClass (Variables|Default|GetTargetSpawn) (Math|Conversions|ToTransform(Vector) (Transformation|GetWorldLocation (Variables|Default|GetDefaultSceneRoot))) "AdjustIfPossibleButDontSpawnIfColliding" "MultiplyWithRoot" 0 0))
          (Variables|/Game/Core/Enemies/BP_Enemy.BP_Enemy_C|SetManager _returnvalue (Variables|Default|GetEnemy%20Manager)))
        (:then_1
          (Variables|Default|SetCurrentSpawns (+ (Variables|Default|GetCurrentSpawns) 1)))
        (:then_2
          (goto _label))))))

(fn ConstructionScript)

(fn InjectManager
  (params (Enemy%20Manager :type BP%20Enemy%20Manager%20Object%20Reference))
  (Variables|Default|SetEnemy%20Manager Enemy%20Manager))